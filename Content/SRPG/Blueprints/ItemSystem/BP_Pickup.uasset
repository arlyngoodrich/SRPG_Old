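; BP_Pickup is a world item pickup that adds its ItemData to the inventory of an actor that touches or interacts with it.
; Both the interactable component's trigger and the PickupSphere overlap find an InventoryContainer and call AutoAddItem.
; The pickup destroys itself when bHasLeftOver returns true and otherwise updates its item information with the remaining item, which appears inverted relative to the flag's name.
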(event OnComponentBeginOverlap(PickupSphere)
  (params (OverlappedComponent :type Primitive%20Component%20Object%20Reference) (OtherActor :type Actor%20Object%20Reference) (OtherComp :type Primitive%20Component%20Object%20Reference) (OtherBodyIndex :type Integer) (bFromSweep :type Boolean) (SweepResult :type Hit%20Result%20Structure%20%28by%20ref%29))
  (bind _returnvalue (Actor|GetComponentbyClass OtherActor "/Script/InventorySystem.InventoryContainer"))
  (Utilities|IsValid _returnvalue
    (:Is%20Valid
      (bind (_outbhasleftover _outremainingitem) (Class|InventoryContainer|AutoAddItem _returnvalue (Variables|Default|GetItemData)))
      (if _outbhasleftover
        (Actor|DestroyActor)
        (else
          (Class|ItemBase|UpdateItemInformation _outremainingitem))))))

(event Custom|On%20Interaction%20Triggered
  (params (Player%20Interaction%20Sensor :type BPC%20Player%20Interaction%20Sensor%20Object%20Reference))
  (bind _returnvalue (Components|GetOwner Player%20Interaction%20Sensor))
  (bind _returnvalue_2 (Actor|GetComponentbyClass _returnvalue "/Script/InventorySystem.InventoryContainer"))
  (Utilities|IsValid _returnvalue_2
    (:Is%20Valid
      (bind (_outbhasleftover _outremainingitem) (Class|InventoryContainer|AutoAddItem _returnvalue_2 (Variables|Default|GetItemData)))
      (if _outbhasleftover
        (Actor|DestroyActor)
        (else
          (Class|ItemBase|UpdateItemInformation _outremainingitem))))))

(event EventBeginPlay
  (EventDispatchers|BindEventtoInteractionTriggered (Variables|Default|GetBPC_InteractableObjectComponent) (delegate Custom|On%20Interaction%20Triggered)))

(fn ConstructionScript)