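; BP_Storage is a multiplayer interactable storage actor that lets a player open a UI for its InventoryContainer.
; Interaction on an unowned storage makes the character its owner and disables their movement; other characters are ignored while owned.
; The InteractingCharacter RepNotify binds menu events on the locally controlled player and toggles storage to open WBP_StorageUI.
; Closing removes the widget, unbinds the events, clears ownership and restores walking.
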(event Custom|Interaction%20Triggered
  (params (Player%20Interaction%20Sensor :type BPC%20Player%20Interaction%20Sensor%20Object%20Reference))
  (bind _returnvalue (Components|GetOwner))
  (bind _owningcharacter (Variables|/InteractionSystem/BPC_PlayerInteractionSensor.BPC_PlayerInteractionSensor_C|GetOwningCharacter Player%20Interaction%20Sensor))
  (if (== _returnvalue 0)
    (Actor|SetOwner _owningcharacter)
    (bind _asbp_player_character (Utilities|Casting|CastToBP_PlayerCharacter _owningcharacter))
    (Variables|References|SetInteracting%20Character _asbp_player_character)
    (Pawn|Components|CharacterMovement|DisableMovement (Variables|/Script/Engine.Character|GetCharacterMovement (Variables|References|GetInteracting%20Character)))
    (elif (== _owningcharacter _returnvalue)
      (Default|ToggleStorage (Variables|References|GetInteracting%20Character)))))

(event Custom|Client%20Add%20Storage%20UI
  (bind _interacting_character (Variables|References|GetInteracting%20Character))
  (Utilities|IsValid (Variables|References|GetInteracting%20Character)
    (:Is%20Valid
      (if (Pawn|IsLocallyControlled (Variables|References|GetInteracting%20Character))
        (EventDispatchers|BindEventtoMenuOpen _interacting_character (delegate Custom|Open%20Storage%20UI))
        (EventDispatchers|BindEventtoMenuClosed _interacting_character (delegate Custom|Remove%20Storage%20UI))
        (Default|ToggleStorage (Variables|References|GetInteracting%20Character))))))

(event Custom|Open%20Storage%20UI
  (bind _returnvalue (UserInterface|CreateWidget "/Game/TestContent/UI/WBP_StorageUI.WBP_StorageUI_C" 0 (Variables|Default|GetInventoryContainer)))
  (bind _output_get (Variables|References|SetStorage%20UI _returnvalue))
  (Default|Initalize _output_get)
  (UserInterface|Viewport|AddtoViewport _output_get 0))

(event Custom|Remove%20Storage%20UI
  (bind _interacting_character (Variables|References|GetInteracting%20Character))
  (if (Pawn|IsLocallyControlled _interacting_character)
    (Widget|RemovefromParent (Variables|References|GetStorage%20UI))
    (CallFunction|ClearOwner)
    (EventDispatchers|UnbindallEventsfromMenuOpen _interacting_character)
    (EventDispatchers|UnbindallEventsfromMenuClosed _interacting_character)))

(event Custom|Clear%20Owner
  (Actor|SetOwner 0)
  (Pawn|Components|CharacterMovement|SetMovementMode (Variables|/Script/Engine.Character|GetCharacterMovement (Variables|References|GetInteracting%20Character)) "MOVE_Walking" 0))

(event EventBeginPlay
  (EventDispatchers|BindEventtoInteractionTriggered (Variables|Default|GetBPC_InteractableObjectComponent) (delegate Custom|Interaction%20Triggered)))

(fn ConstructionScript)

(fn OnRepInteractingCharacter
  (CallFunction|ClientAddStorageUI))