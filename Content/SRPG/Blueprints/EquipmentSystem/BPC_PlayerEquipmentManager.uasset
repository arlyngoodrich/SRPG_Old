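; Player equipment manager component that lets the owning BP_PlayerCharacter equip and attack with an ax.
; Slot 1 toggles the weapon, spawning BP_Ax onto the left-hand mesh socket or destroying it.
; The primary action passes through PrimaryMulticast to play a two-handed swing montage, whose notifies start and end weapon damage only with authority.
; The secondary action is an empty stub.
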(event Custom|Primary%20Called
  (CallFunction|PrimaryMulticast))

(event Custom|Secondary%20Called)

(event Custom|Slot%201%20Called
  (Utilities|IsValid (Variables|Default|GetAttached%20Primary)
    (:Is%20Valid
      (Actor|DestroyActor (Variables|Default|GetAttached%20Primary))
      (Variables|Default|SetPrimary%20Attached false))
    (:Is%20Not%20Valid
      (bind _returnvalue (Game|SpawnActorfromClass "/Game/SRPG/TestingContent/Blueprints/BP_Ax.BP_Ax_C" (Math|Transform|MakeTransform "0, 0, 0" "0, 0, 0" "1,1,1") "Undefined" (Variables|Components|GetMy%20Character) 0))
      (bind _output_get (Variables|Default|SetAttached%20Primary _returnvalue))
      (Transformation|AttachComponentToComponent _output_get (Variables|Default|GetMesh) "Hand_LSocket" "SnapToTarget" "SnapToTarget" "KeepRelative" true)
      (Variables|Default|SetPrimary%20Attached true))))

(event Custom|Primary%20Multicast
  (bind _attached_primary (Variables|Default|GetAttached%20Primary))
  (if (Variables|Default|GetPrimary%20Attached)
    (bind _notifyname (Animation|Montage|PlayMontage (Variables|Default|GetMesh) "/Game/SRPG/TestingContent/Animations/AM_TwoHandedSwing.AM_TwoHandedSwing")
      (:OnNotifyBegin
        (if (Ability|HasAuthority (Variables|Components|GetMy%20Character))
          (if (Utilities|Name|Equal(Name) _notifyname "Start Damage")
            (Utilities|IsValid _attached_primary
              (:Is%20Valid
                (Default|StartDamage _attached_primary)))
            (elif (Utilities|Name|Equal(Name) _notifyname "End Damage")
              (Utilities|IsValid _attached_primary
                (:Is%20Valid
                  (Default|EndDamage _attached_primary))))))))))

(event EventBeginPlay
  (bind _asbp_player_character (Utilities|Casting|CastToBP_PlayerCharacter (Components|GetOwner)))
  (bind _output_get (Variables|Components|SetMy%20Character _asbp_player_character))
  (Variables|Default|SetMesh (Variables|/Script/Engine.Character|GetMesh _output_get)))