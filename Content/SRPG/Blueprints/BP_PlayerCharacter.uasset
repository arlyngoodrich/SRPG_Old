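; BP_PlayerCharacter is the player character, turning input actions into inventory, interaction and equipment actions.
; On BeginPlay it caches BP_PlayerController and creates the inventory widget, which the inventory input or ToggleStorage shows and hides with matching input mode and cursor.
; Other inputs forward to the interaction sensor, inventory manager and equipment manager components, some also firing dispatchers.
; Primary branches on authority, using PrimaryMulticast on the server and PrimaryCalled on remotes.
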(event Custom|Toggle%20Storage
  (bind _inventory_container_widget (Variables|Components|GetInventory%20Container%20Widget))
  (bind _player_controller (Variables|Components|GetPlayer%20Controller))
  (if (UserInterface|Viewport|IsinViewport _inventory_container_widget)
    (Widget|RemovefromParent _inventory_container_widget)
    (Input|SetInputModeGameOnly _player_controller)
    (Variables|/Script/Engine.PlayerController|SetbShowMouseCursor _player_controller false)
    (Default|CallMenuClosed)
    (else
      (UserInterface|Viewport|AddtoViewport (Variables|Components|GetInventory%20Container%20Widget) 0)
      (Input|SetInputModeGameandUI _player_controller 0 "LockInFullscreen" true)
      (Variables|/Script/Engine.PlayerController|SetbShowMouseCursor _player_controller true)
      (Default|CallMenuOpen))))

(event EventBeginPlay
  (CallFunction|Initalize))

(event Input|ActionEvents|InputActionToggleInventory
  (params (Key :type Key%20Structure :default "None"))
  (bind _inventory_container_widget (Variables|Components|GetInventory%20Container%20Widget))
  (bind _player_controller (Variables|Components|GetPlayer%20Controller))
  (:Pressed
    (if (UserInterface|Viewport|IsinViewport _inventory_container_widget)
      (Widget|RemovefromParent _inventory_container_widget)
      (Input|SetInputModeGameOnly _player_controller)
      (Variables|/Script/Engine.PlayerController|SetbShowMouseCursor _player_controller false)
      (Default|CallMenuClosed)
      (else
        (UserInterface|Viewport|AddtoViewport (Variables|Components|GetInventory%20Container%20Widget) 0)
        (Input|SetInputModeGameandUI _player_controller 0 "LockInFullscreen" true)
        (Variables|/Script/Engine.PlayerController|SetbShowMouseCursor _player_controller true)
        (Default|CallMenuOpen)))))

(event Input|ActionEvents|InputActionRotateInventoryItem
  (params (Key :type Key%20Structure :default "None"))
  (:Pressed
    (Default|PlayerPressedRotate (Variables|Default|GetBPC_PlayerInventoryManager))))

(event Input|ActionEvents|InputActionInteract
  (params (Key :type Key%20Structure :default "None"))
  (:Pressed
    (Default|Interact (Variables|Default|GetBPC_PlayerInteractionSensor))))

(event Input|ActionEvents|InputActionPrimary
  (params (Key :type Key%20Structure :default "None"))
  (bind _bpc_playerequipmentmanager (Variables|Default|GetBPC_PlayerEquipmentManager))
  (:Pressed
    (Default|CallPrimaryCalled)
    (Networking|SwitchHasAuthority
      (:Authority
        (Default|PrimaryMulticast _bpc_playerequipmentmanager))
      (:Remote
        (Default|PrimaryCalled _bpc_playerequipmentmanager)))))

(event Input|ActionEvents|InputActionSecondary
  (params (Key :type Key%20Structure :default "None"))
  (:Pressed
    (Default|CallSecondaryCalled)
    (Default|SecondaryCalled (Variables|Default|GetBPC_PlayerEquipmentManager))))

(event Input|ActionEvents|InputActionUseSlot1
  (params (Key :type Key%20Structure :default "None"))
  (:Pressed
    (Default|CallUseSlot1)
    (Default|Slot1Called (Variables|Default|GetBPC_PlayerEquipmentManager))))

(fn ConstructionScript
  (|CallParentFunction))

(fn Initalize
  (bind _asbp_player_controller (Utilities|Casting|CastToBP_PlayerController (Pawn|GetController)))
  (Variables|Components|SetPlayer%20Controller _asbp_player_controller)
  (bind _returnvalue (UserInterface|CreateWidget "/InventorySystem/WBP_InventoryContainer.WBP_InventoryContainer_C" 0 (Variables|Default|GetInventoryContainer)))
  (Variables|Components|SetInventory%20Container%20Widget _returnvalue))