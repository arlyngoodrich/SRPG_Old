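; BP_TestTreeFoliage is a test tree foliage Blueprint that turns into wood pickups when depleted.
; On depletion, the authority swaps the mesh to a low-poly trunk and, after a delay, caches world transforms of components tagged LogSpawner.
; It then destroys the foliage mesh component and spawns a BP_TestPickupWood at each cached transform.
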(event EventBeginPlay)

(event EventBPEonFoliageDepleted
  (Networking|SwitchHasAuthority
    (:Authority
      (Components|StaticMesh|SetStaticMesh (Variables|Default|GetFoliageMeshComponent) "/Game/TestContent/Meshes/SM_Trunk_LP.SM_Trunk_LP")
      (Utilities|FlowControl|Delay 2.0)
      (for _array_element (Actor|GetComponentsbyTag "/Script/Engine.SceneComponent" "LogSpawner")
        (Utilities|Array|Add (Variables|Default|GetSpawn%20Transforms) (Transformation|GetWorldTransform _array_element)))
      (Utilities|FlowControl|Delay 0.001)
      (Components|DestroyComponent (Variables|Default|GetFoliageMeshComponent))
      (for _array_element_2 (Variables|Default|GetSpawn%20Transforms)
        (Game|SpawnActorfromClass "/Game/TestContent/Blueprints/BP_TestPickupWood.BP_TestPickupWood_C" _array_element_2 "Undefined" 0 0)))))

(fn ConstructionScript)